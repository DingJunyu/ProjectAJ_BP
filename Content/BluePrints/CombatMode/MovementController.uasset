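; MovementController is a combat-mode actor that tracks a selected player piece and grid cell, then moves the piece onto that cell.
; SetPlayerSelected toggles the piece; SetGridSelected requires one, moving it when the same grid is picked twice.
; The grid move teleports by setting location, then clears both selections.
; A MovementTest input nudges the piece by random X/Y offsets, and Tick prints the selection through a delayed debug macro.
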(event `self.ReceiveBeginPlay`
  (`self.EnableInput` (`GameplayStatics.GetPlayerController` 0)))

(event `self.ReceiveTick`
  (params (DeltaSeconds :type "Float (single-precision)"))
  (`self.Debug`))

(event `InputAction|MovementTest`
  (params (Key :type "Key Structure"))
  (:`Pressed`
    (`KismetSystemLibrary.PrintText` "Hello2" :!label _label)
    (`self.GetMovementPos`)
    (`self.MovePlayer`))
  (:`Released`
    (goto _label)))

(fn `SetGridSelected`
  (params (SelectedGrid :type "/Game/BluePrints/CombatMode/Enviroments/BP_StandardMapGrid Object Reference"))
  (if (`KismetSystemLibrary.IsValid` (`self.SelectedPlayer`))
    (if (== (`self.SelectedGrid`) SelectedGrid)
      (`self.MovePlayer_ByGrid`)
      (else
        (set `self.SelectedGrid` SelectedGrid)))
    (else
      (`KismetSystemLibrary.PrintText` "You need to select Something"))))

(fn `SetPlayerSelected`
  (params (SelectedPlayer :type "/Game/BluePrints/CombatMode/Characters/Player Object Reference"))
  (if (== SelectedPlayer (`self.SelectedPlayer`))
    (bind _output_get (set `self.SelectedPlayer` null))
    (`KismetSystemLibrary.PrintText` (`KismetTextLibrary.Conv_StringToText` (`KismetStringLibrary.Concat_StrStr` (`KismetSystemLibrary.GetObjectName` _output_get) " Selected")))
    (else
      (bind _output_get_2 (set `self.SelectedPlayer` SelectedPlayer))
      (`KismetSystemLibrary.PrintText` (`KismetTextLibrary.Conv_StringToText` (`KismetStringLibrary.Concat_StrStr` (`KismetSystemLibrary.GetObjectName` _output_get_2) " UnSelected"))))))

(fn `UserConstructionScript`)